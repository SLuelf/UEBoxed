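; Tiltable box that acts as a Learning Agents agent, apparently for learning to balance a ball.
; On BeginPlay it registers with the tagged LearningAgentsManager and stores its agent ID.
; SetBoxRotX and SetBoxRotY step roll and pitch toward targets at constant speed, throttled by a shared counter that only the X setter advances.
; ResetBall repositions the ball above the box, zeroes its velocities and gives the box a small random tilt.
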(event `self.ReceiveBeginPlay`
  (bind _outactors (`GameplayStatics.GetAllActorsWithTag` "LearningAgentsManager"))
  (for _array_element _outactors
    (bind _returnvalue (`self.GetComponentByClass` _array_element "/Script/LearningAgents.LearningAgentsManager"))
    (`/Engine/EditorBlueprintResources/StandardMacros.IsValid` _returnvalue
      (:`Is Valid`
        (bind _returnvalue_2 (`LearningAgentsManager.AddAgent` _returnvalue self))
        (set `self.AgentID` _returnvalue_2)
        (set `self.FoundManager` true)
        (set `self.TickCounter` 0))))
  (if (not (`self.FoundManager`))
    (`KismetSystemLibrary.PrintString` "Could not find the Learning Agents manager.")))

(event `self.ReceiveTick`
  (params (DeltaSeconds :type "Float (single-precision)")))

(fn `ResetBall`
  (bind _returnvalue (`self.GetComponentByClass` (`self.BallVar`) "/Script/Engine.StaticMeshComponent"))
  (`SceneComponent.K2_SetRelativeLocation` _returnvalue (`KismetMathLibrary.TransformLocation` (`KismetMathLibrary.Conv_VectorToTransform` (`self.K2_GetActorLocation`)) (0.0 0.0 100.0)) false false)
  (`PrimitiveComponent.SetPhysicsLinearVelocity` _returnvalue (0.0 0.0 0.0) false "None")
  (`PrimitiveComponent.SetPhysicsAngularVelocityInDegrees` _returnvalue (0.0 0.0 0.0) false "None")
  (`self.K2_SetActorRotation` (`KismetMathLibrary.ComposeRotators` (`KismetMathLibrary.RotatorFromAxisAndAngle` (1.0 0.0 0.0) (`KismetMathLibrary.RandomFloatInRange` -5.0 5.0)) (`KismetMathLibrary.RotatorFromAxisAndAngle` (0.0 1.0 0.0) (`KismetMathLibrary.RandomFloatInRange` -5.0 5.0)))))

(fn `SetBoxRotX`
  (params (RotationX :type "Float (double-precision)"))
  (bind _returnvalue (`SceneComponent.GetSocketRotation` (`self.Cube`) "None"))
  (if (== (mod (`self.TickCounter`) 6) 0)
    (`self.K2_SetActorRotation` (`KismetMathLibrary.RInterpTo_Constant` _returnvalue (`KismetMathLibrary.MakeRotator` RotationX (.pitch _returnvalue)) (`GameplayStatics.GetWorldDeltaSeconds`) 50.0)))
  (set `self.TickCounter` (+ (`self.TickCounter`) 1)))

(fn `SetBoxRotY`
  (params (RotationY :type "Float (double-precision)"))
  (bind _returnvalue (`SceneComponent.GetSocketRotation` (`self.Cube`) "None"))
  (if (== (mod (`self.TickCounter`) 6) 0)
    (`self.K2_SetActorRotation` (`KismetMathLibrary.RInterpTo_Constant` _returnvalue (`KismetMathLibrary.MakeRotator` (.roll _returnvalue) RotationY) (`GameplayStatics.GetWorldDeltaSeconds`) 50.0))))

(fn `UserConstructionScript`)