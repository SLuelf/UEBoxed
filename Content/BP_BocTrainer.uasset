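; Learning Agents trainer that teaches BP_Box agents to keep a ball balanced on top of the box.
; Reward is a small constant, minus a penalty when the ball is not above the box or drifts out along X; the Y check compares the box with itself, so never triggers.
; Episodes terminate when the ball drifts out on X or Y or sits slightly below the box.
; Episode reset calls ResetBall on the box.
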(fn `GatherAgentCompletion`
  (params (AgentId :type Integer))
  (returns (OutCompletion :type "ELearningAgentsCompletion Enum"))
  (locals (CompletionActor :type "/Game/Blueprints/BP_Box Object Reference"))
  (set `local.CompletionActor` (`self.GetAgent` AgentId "/Game/Blueprints/BP_Box.BP_Box_C"))
  (return (`LearningAgentsCompletions.MakeCompletionOnCondition` (or (or (not (`KismetMathLibrary.InRange_FloatFloat` (- (.y (`Actor.K2_GetActorLocation` (`local.CompletionActor`))) (.y (`SceneComponent.GetSocketLocation` (`Actor.GetComponentByClass` (`/Game/Blueprints/BP_Box.BallVar` (`local.CompletionActor`)) "/Script/Engine.StaticMeshComponent") "None"))) -80.0 80.0)) (not (`KismetMathLibrary.InRange_FloatFloat` (- (.x (`Actor.K2_GetActorLocation` (`local.CompletionActor`))) (.x (`SceneComponent.GetSocketLocation` (`Actor.GetComponentByClass` (`/Game/Blueprints/BP_Box.BallVar` (`local.CompletionActor`)) "/Script/Engine.StaticMeshComponent") "None"))) -80.0 80.0))) (`KismetMathLibrary.InRange_FloatFloat` (- (.z (`SceneComponent.GetSocketLocation` (`Actor.GetComponentByClass` (`/Game/Blueprints/BP_Box.BallVar` (`local.CompletionActor`)) "/Script/Engine.StaticMeshComponent") "None")) (.z (`Actor.K2_GetActorLocation` (`local.CompletionActor`)))) -200.0 0.0)) "Termination" "ConditionCompletion" false null)))

(fn `GatherAgentReward`
  (params (AgentId :type Integer))
  (returns (OutReward :type "Float (single-precision)"))
  (locals (RewardActor :type "/Game/Blueprints/BP_Box Object Reference") (Penalty :type Boolean))
  (bind _y (.y (`Actor.K2_GetActorLocation` (`local.RewardActor`))))
  (set `local.RewardActor` (`self.GetAgent` AgentId "/Game/Blueprints/BP_Box.BP_Box_C"))
  (set `local.Penalty` false)
  (`/Engine/EditorBlueprintResources/StandardMacros.CompareFloat` (.z (`SceneComponent.GetSocketLocation` (`Actor.GetComponentByClass` (`/Game/Blueprints/BP_Box.BallVar` (`local.RewardActor`)) "/Script/Engine.StaticMeshComponent") "None")) (.z (`Actor.K2_GetActorLocation` (`local.RewardActor`)))
    (:`>`
      (if (or (not (`KismetMathLibrary.InRange_FloatFloat` (- _y _y) -80.0 80.0)) (not (`KismetMathLibrary.InRange_FloatFloat` (- (.x (`Actor.K2_GetActorLocation` (`local.RewardActor`))) (.x (`SceneComponent.GetSocketLocation` (`Actor.GetComponentByClass` (`/Game/Blueprints/BP_Box.BallVar` (`local.RewardActor`)) "/Script/Engine.StaticMeshComponent") "None"))) -80.0 80.0)))
        (bind _output_get (set `local.Penalty` true :!label _label))))
    (:`==`
      (goto _label))
    (:`<`
      (goto _label)))
  (return (+ (`LearningAgentsRewards.MakeReward` 0.1 1.0 "Reward" false null) (`LearningAgentsRewards.MakeRewardOnCondition` _output_get -1.0 "ConditionReward" false null))))

(fn `ResetAgentEpisode`
  (params (AgentId :type Integer))
  (`/Game/Blueprints/BP_Box.ResetBall` (`self.GetAgent` AgentId "/Game/Blueprints/BP_Box.BP_Box_C")))