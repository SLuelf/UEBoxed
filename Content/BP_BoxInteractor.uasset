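; BP_BoxInteractor is a Learning Agents interactor that lets an agent control a BP_Box's tilt in response to its ball.
; Observations are nested structs of the box cube's roll and pitch plus the ball's box-relative position and physics velocity, built from scaled floats.
; Actions are two floats, scaled as rotations and passed to the box's SetBoxRotX and SetBoxRotY.
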(fn `GatherAgentObservation`
  (params (InObservationObject :type "LearningAgentsObservationObject Object Reference") (AgentId :type Integer))
  (returns (OutObservationObjectElement :type "LearningAgentsObservationObjectElement Structure"))
  (locals (ObsActor :type "/Game/Blueprints/BP_Box Object Reference"))
  (bind _obsactor (`local.ObsActor`))
  (bind _returnvalue (`Actor.GetComponentByClass` (`/Game/Blueprints/BP_Box.BallVar` _obsactor) "/Script/Engine.StaticMeshComponent"))
  (set `local.ObsActor` (`self.GetAgent` AgentId "/Game/Blueprints/BP_Box.BP_Box_C"))
  (bind _returnvalue_2 (`PrimitiveComponent.GetPhysicsLinearVelocity` _returnvalue "None"))
  (return (`LearningAgentsObservations.MakeStructObservation` (`local.InObservationObject`) (`|MakeMap` "Box" (`LearningAgentsObservations.MakeStructObservation` (`local.InObservationObject`) (`|MakeMap` "CurrRotX" (`LearningAgentsObservations.MakeFloatObservation` (`local.InObservationObject`) (.roll (`SceneComponent.GetSocketRotation` (`/Game/Blueprints/BP_Box.Cube` (`local.ObsActor`)) "None")) 1.0 "CurrBoxXRot" false null) "CurrRotY" (`LearningAgentsObservations.MakeFloatObservation` (`local.InObservationObject`) (.pitch (`SceneComponent.GetSocketRotation` (`/Game/Blueprints/BP_Box.Cube` (`local.ObsActor`)) "None")) 1.0 "CurrBoxYRot" false null) :!type "Name") "BoxObservation") "Ball" (`LearningAgentsObservations.MakeStructObservation` (`local.InObservationObject`) (`|MakeMap` "Position" (`LearningAgentsObservations.MakeStructObservation` (`local.InObservationObject`) (`|MakeMap` "XRelPos" (`LearningAgentsObservations.MakeFloatObservation` (`local.InObservationObject`) (- (.x (`SceneComponent.GetSocketLocation` _returnvalue "None")) (.x (`SceneComponent.GetSocketLocation` (`Actor.GetComponentByClass` _obsactor "/Script/Engine.StaticMeshComponent") "None"))) 100.0 "XBallPos" false null) "YRelPos" (`LearningAgentsObservations.MakeFloatObservation` (`local.InObservationObject`) (- (.y (`SceneComponent.GetSocketLocation` _returnvalue "None")) (.y (`SceneComponent.GetSocketLocation` (`Actor.GetComponentByClass` _obsactor "/Script/Engine.StaticMeshComponent") "None"))) 100.0 "YBallPos" false null) "ZRelPos" (`LearningAgentsObservations.MakeFloatObservation` (`local.InObservationObject`) (- (.z (`SceneComponent.GetSocketLocation` _returnvalue "None")) (.z (`SceneComponent.GetSocketLocation` (`Actor.GetComponentByClass` _obsactor "/Script/Engine.StaticMeshComponent") "None"))) 100.0 "ZBallPos" false null) :!type "Name") "BallPosition") "Velocity" (`LearningAgentsObservations.MakeStructObservation` (`local.InObservationObject`) (`|MakeMap` "XVel" (`LearningAgentsObservations.MakeFloatObservation` (`local.InObservationObject`) (.x _returnvalue_2) 200.0 "XBallVel" false null) "YVel" (`LearningAgentsObservations.MakeFloatObservation` (`local.InObservationObject`) (.y _returnvalue_2) 200.0 "YBallVel" false null) "ZVel" (`LearningAgentsObservations.MakeFloatObservation` (`local.InObservationObject`) (.z _returnvalue_2) 200.0 "ZBallVel" false null) :!type "Name") "BallVelocity") :!type "Name") "BallObservation") :!type "Name"))))

(fn `PerformAgentAction`
  (params (InActionObject :type "LearningAgentsActionObject Object Reference") (InActionObjectElement :type "LearningAgentsActionObjectElement Structure (by ref)") (AgentId :type Integer))
  (set `self.ActActor` (`self.GetAgent` AgentId "/Game/Blueprints/BP_Box.BP_Box_C"))
  (bind _outelements (`LearningAgentsActions.GetStructAction` (`local.InActionObject`) (`local.InActionObjectElement`)))
  (`|ExecutionSequence`
    (:`then_0`
      (bind _outvalue (`LearningAgentsActions.GetFloatAction` (`local.InActionObject`) (`BlueprintMapLibrary.Map_Find` _outelements "FutRotX") 45.0 "FloatAction" false null))
      (`/Game/Blueprints/BP_Box.SetBoxRotX` (`self.ActActor`) _outvalue))
    (:`then_1`
      (bind _outvalue_2 (`LearningAgentsActions.GetFloatAction` (`local.InActionObject`) (`BlueprintMapLibrary.Map_Find` _outelements "FutRotY") 45.0 "FloatAction" false null))
      (`/Game/Blueprints/BP_Box.SetBoxRotY` (`self.ActActor`) _outvalue_2))))

(fn `SpecifyAgentAction`
  (params (InActionSchema :type "LearningAgentsActionSchema Object Reference"))
  (returns (OutActionSchemaElement :type "LearningAgentsActionSchemaElement Structure"))
  (return (`LearningAgentsActions.SpecifyStructAction` (`local.InActionSchema`) (`|MakeMap` "FutRotX" (`LearningAgentsActions.SpecifyFloatAction` (`local.InActionSchema`)) "FutRotY" (`LearningAgentsActions.SpecifyFloatAction` (`local.InActionSchema`)) :!type "Name"))))

(fn `SpecifyAgentObservation`
  (params (InObservationSchema :type "LearningAgentsObservationSchema Object Reference"))
  (returns (OutObservationSchemaElement :type "LearningAgentsObservationSchemaElement Structure"))
  (return (`LearningAgentsObservations.SpecifyStructObservation` (`local.InObservationSchema`) (`|MakeMap` "Box" (`LearningAgentsObservations.SpecifyStructObservation` (`local.InObservationSchema`) (`|MakeMap` "CurrRotX" (`LearningAgentsObservations.SpecifyFloatObservation` (`local.InObservationSchema`) "CurrBoxXRot") "CurrRotY" (`LearningAgentsObservations.SpecifyFloatObservation` (`local.InObservationSchema`) "CurrBoxYRot") :!type "Name") "BoxObservation") "Ball" (`LearningAgentsObservations.SpecifyStructObservation` (`local.InObservationSchema`) (`|MakeMap` "Position" (`LearningAgentsObservations.SpecifyStructObservation` (`local.InObservationSchema`) (`|MakeMap` "XRelPos" (`LearningAgentsObservations.SpecifyFloatObservation` (`local.InObservationSchema`) "XBallPos") "YRelPos" (`LearningAgentsObservations.SpecifyFloatObservation` (`local.InObservationSchema`) "YBallPos") "ZRelPos" (`LearningAgentsObservations.SpecifyFloatObservation` (`local.InObservationSchema`) "ZBallPos") :!type "Name") "BallPosition") "Velocity" (`LearningAgentsObservations.SpecifyStructObservation` (`local.InObservationSchema`) (`|MakeMap` "XVel" (`LearningAgentsObservations.SpecifyFloatObservation` (`local.InObservationSchema`) "XBallVel") "YVel" (`LearningAgentsObservations.SpecifyFloatObservation` (`local.InObservationSchema`) "YBallVel") "ZVel" (`LearningAgentsObservations.SpecifyFloatObservation` (`local.InObservationSchema`) "ZBallVel") :!type "Name") "BallVelocity") :!type "Name") "BallObservation") :!type "Name"))))